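; Villager NPC that turns to face the player and acts as a quest end point for obtaining a diamond sword.
; Tick yaws the mesh and rotates its widget toward the player, hiding the widget once a waiting villager is interacted with.
; A sphere overlap toggles prompt text as the player enters or leaves.
; Holding the sword switches the conversation; once finished, a completion flag is saved, re-written every tick.
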(event `self.ReceiveTick`
  (params (DeltaSeconds :type "Float (single-precision)"))
  (bind _widget (`self.Widget`))
  (bind (_returnvalue_location _returnvalue_rotation _returnvalue_scale) (`KismetMathLibrary.BreakTransform` (`SceneComponent.K2_GetComponentToWorld` _widget)))
  (bind _returnvalue (`KismetMathLibrary.FindLookAtRotation` (`self.K2_GetActorLocation` (`GameplayStatics.GetPlayerCharacter` 0)) (`self.K2_GetActorLocation`)))
  (`self.CheckDiamondSword`)
  (`SceneComponent.K2_SetWorldTransform` _widget (`KismetMathLibrary.MakeTransform` _returnvalue_location (`KismetMathLibrary.MakeRotator` (.roll _returnvalue) (.pitch _returnvalue) (+ (.yaw _returnvalue) 180.0)) _returnvalue_scale) false false)
  (`SceneComponent.K2_SetRelativeRotation` (`self.StaticMesh`) (`KismetMathLibrary.MakeRotator` 0.0 0.0 (+ (.yaw _returnvalue) 180.0)) false false)
  (if (and (`self.IsInteracted`) (`self.isWaiting`))
    (set `self.isWaiting` false)
    (`SceneComponent.SetVisibility` (`self.Widget`) false false)))

(event `self.Sphere.OnComponentBeginOverlap`
  (params (OverlappedComponent :type "PrimitiveComponent Object Reference") (OtherActor :type "Actor Object Reference") (OtherComp :type "PrimitiveComponent Object Reference") (OtherBodyIndex :type Integer) (bFromSweep :type Boolean) (SweepResult :type "HitResult Structure (by ref)"))
  (cast `UltraMinecraftCharacter` OtherActor)
  (`self.ShowText`)
  (set `self.isOverlap` true))

(event `self.Sphere.OnComponentEndOverlap`
  (params (OverlappedComponent :type "PrimitiveComponent Object Reference") (OtherActor :type "Actor Object Reference") (OtherComp :type "PrimitiveComponent Object Reference") (OtherBodyIndex :type Integer))
  (cast `UltraMinecraftCharacter` OtherActor)
  (`self.ShowText`)
  (set `self.isOverlap` false))

(fn `CheckDiamondSword`
  (bind _asfirst_person_character (cast `/Game/FirstPersonCPP/Blueprints/FirstPersonCharacter` (`GameplayStatics.GetPlayerCharacter` 0)))
  (if (`UltraMinecraftCharacter.HaveWieldableItemInInventory` _asfirst_person_character "/Game/Assets/Blueprints/Wieldables/Weapons/Sword/Wieldable_Tool_Sword_Diamond.Wieldable_Tool_Sword_Diamond_C")
    (`self.ChangeConversation` 2)
    (if (`self.isFinishConversation`)
      (bind _returnvalue (`GameplayStatics.CreateSaveGameObject` "/Game/Assets/Levels/SaveGameData.SaveGameData_C"))
      (set `/Game/Assets/Levels/SaveGameData.isFinish` true _returnvalue)
      (`GameplayStatics.SaveGameToSlot` _returnvalue "Minecraft"))))

(fn `ShowText`
  (`SceneComponent.SetVisibility` (`self.TextRender`) (`self.isVisible`) false)
  (set `self.isVisible` (not (`self.isVisible`))))

(fn `UserConstructionScript`)